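; Clinic minigame reference book actor that displays pages as widgets on four surfaces: left, right, and the front and back of a turning page.
; InitializePages creates a WBP_ClinicReferencePage for each surface for the given player, passing it the book and a surface index.
; RefreshPages has each surface's page widget re-render itself, so page content logic lives in the widget rather than here.
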(event EventInitializePages
  (params (Player :type Player%20Controller%20Object%20Reference))
  (bind _self self)
  (bind _returnvalue (UserInterface|CreateWidget "/Game/Minigames/Clinic/UI/WBP_ClinicReferencePage.WBP_ClinicReferencePage_C" Player))
  (Variables|/Game/Minigames/Clinic/UI/WBP_ClinicReferencePage.WBP_ClinicReferencePage_C|SetBook _returnvalue _self)
  (Variables|/Game/Minigames/Clinic/UI/WBP_ClinicReferencePage.WBP_ClinicReferencePage_C|SetSurfaceIndex _returnvalue 0)
  (UserInterface|SetWidget (Variables|Default|GetLeftPage) _returnvalue)
  (bind _returnvalue_2 (UserInterface|CreateWidget "/Game/Minigames/Clinic/UI/WBP_ClinicReferencePage.WBP_ClinicReferencePage_C" Player))
  (Variables|/Game/Minigames/Clinic/UI/WBP_ClinicReferencePage.WBP_ClinicReferencePage_C|SetBook _returnvalue_2 _self)
  (Variables|/Game/Minigames/Clinic/UI/WBP_ClinicReferencePage.WBP_ClinicReferencePage_C|SetSurfaceIndex _returnvalue_2 1)
  (UserInterface|SetWidget (Variables|Default|GetRightPage) _returnvalue_2)
  (bind _returnvalue_3 (UserInterface|CreateWidget "/Game/Minigames/Clinic/UI/WBP_ClinicReferencePage.WBP_ClinicReferencePage_C" Player))
  (Variables|/Game/Minigames/Clinic/UI/WBP_ClinicReferencePage.WBP_ClinicReferencePage_C|SetBook _returnvalue_3 _self)
  (Variables|/Game/Minigames/Clinic/UI/WBP_ClinicReferencePage.WBP_ClinicReferencePage_C|SetSurfaceIndex _returnvalue_3 2)
  (UserInterface|SetWidget (Variables|Default|GetTurningPageFront) _returnvalue_3)
  (bind _returnvalue_4 (UserInterface|CreateWidget "/Game/Minigames/Clinic/UI/WBP_ClinicReferencePage.WBP_ClinicReferencePage_C" Player))
  (Variables|/Game/Minigames/Clinic/UI/WBP_ClinicReferencePage.WBP_ClinicReferencePage_C|SetBook _returnvalue_4 _self)
  (Variables|/Game/Minigames/Clinic/UI/WBP_ClinicReferencePage.WBP_ClinicReferencePage_C|SetSurfaceIndex _returnvalue_4 3)
  (UserInterface|SetWidget (Variables|Default|GetTurningPageBack) _returnvalue_4))

(event EventRefreshPages
  (bind _aswbp_clinic_reference_page (Utilities|Casting|CastToWBP_ClinicReferencePage (UserInterface|GetUserWidgetObject (Variables|Default|GetLeftPage))))
  (Default|RenderPage _aswbp_clinic_reference_page)
  (bind _aswbp_clinic_reference_page_2 (Utilities|Casting|CastToWBP_ClinicReferencePage (UserInterface|GetUserWidgetObject (Variables|Default|GetRightPage))))
  (Default|RenderPage _aswbp_clinic_reference_page_2)
  (bind _aswbp_clinic_reference_page_3 (Utilities|Casting|CastToWBP_ClinicReferencePage (UserInterface|GetUserWidgetObject (Variables|Default|GetTurningPageFront))))
  (Default|RenderPage _aswbp_clinic_reference_page_3)
  (bind _aswbp_clinic_reference_page_4 (Utilities|Casting|CastToWBP_ClinicReferencePage (UserInterface|GetUserWidgetObject (Variables|Default|GetTurningPageBack))))
  (Default|RenderPage _aswbp_clinic_reference_page_4))

(fn ConstructionScript)