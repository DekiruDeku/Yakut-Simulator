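; Clinic minigame computer actor that shows a console UI on an in-world screen.
; On BeginPlay, if its Scenario is valid, it creates a WBP_ClinicConsole with that scenario and assigns it to the ScreenWidget component.
; The construction script fits the screen to the ScreenBounds box, deriving draw height from the box's aspect ratio at fixed draw width, then scaling the widget to the box's size.
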(event EventBeginPlay
  (Utilities|IsValid (Variables|Default|GetScenario)
    (:Is%20Valid
      (bind _returnvalue (UserInterface|CreateWidget "/Game/Minigames/Clinic/UI/WBP_ClinicConsole.WBP_ClinicConsole_C" (Game|GetPlayerController 0) (Variables|Default|GetScenario)))
      (UserInterface|SetWidget (Variables|Default|GetScreenWidget) _returnvalue))))

(event Collision|EventActorBeginOverlap
  (params (OtherActor :type Actor%20Object%20Reference)))

(event EventTick
  (params (DeltaSeconds :type Float%20%28single-precision%29)))

(fn ConstructionScript
  (bind _returnvalue (Math|Float|MakeLiteralFloat 2.0))
  (bind _returnvalue_2 (Math|Float|MakeLiteralFloat 2.0))
  (bind _screenwidget (Variables|Default|GetScreenWidget))
  (bind _screenbounds (Variables|Default|GetScreenBounds))
  (bind _returnvalue_3 (Components|Box|GetScaledBoxExtent _screenbounds))
  (bind _returnvalue_4 (Class|WidgetComponent|GetDrawSize _screenwidget))
  (bind (_x _y _z) (Math|Vector|BreakVector _returnvalue_3))
  (bind _x_2 (Math|Vector2D|BreakVector2D _returnvalue_4))
  (bind _returnvalue_5 (* _y _returnvalue))
  (bind _returnvalue_6 (* _z _returnvalue_2))
  (bind _returnvalue_7 (Math|Float|SafeDivide _returnvalue_6 _returnvalue_5))
  (bind _returnvalue_8 (Math|Float|SafeDivide _returnvalue_5 _x_2))
  (bind _returnvalue_9 (* _x_2 _returnvalue_7))
  (bind _returnvalue_10 (Math|Float|Round _returnvalue_9))
  (bind _returnvalue_11 (Math|Integer|Max(Integer) 1 _returnvalue_10))
  (Class|WidgetComponent|SetDrawSize _screenwidget (Math|Vector2D|MakeVector2D _x_2 (Math|Conversions|ToFloat(Integer) _returnvalue_11)))
  (Transformation|SetWorldScale3D _screenwidget (Math|Vector|MakeVector _returnvalue_8 _returnvalue_8 (Math|Float|SafeDivide _returnvalue_6 (Math|Conversions|ToFloat(Integer) _returnvalue_11)))))