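; VR main HUD that hosts a world-space settings panel and turns trigger input into UI clicks.
; BeginPlay creates WBP_Settings with the game instance and pushes the settings sound mix, which EndPlay pops.
; Holding the X and Y settings inputs together starts a short timer that toggles the panel, placed facing the camera.
; Triggers drive the pawn's pointer clicks with press/release hysteresis, pressing only over widgets and releasing when that hand is busy.
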(event Input|EnhancedActionEvents|EnhancedInputActionIA_SettingsX
  (params (ActionValue :type Boolean) (ElapsedSeconds :type Float%20%28double-precision%29) (TriggeredSeconds :type Float%20%28double-precision%29) (InputAction :type Input%20Action%20Object%20Reference :default "/Game/Base/Input/IA_SettingsX.IA_SettingsX"))
  (:Started
    (CallFunction|SetSettingsX true))
  (:Canceled
    (CallFunction|SetSettingsX false :!label _label))
  (:Completed
    (goto _label)))

(event Input|EnhancedActionEvents|EnhancedInputActionIA_SettingsY
  (params (ActionValue :type Boolean) (ElapsedSeconds :type Float%20%28double-precision%29) (TriggeredSeconds :type Float%20%28double-precision%29) (InputAction :type Input%20Action%20Object%20Reference :default "/Game/Base/Input/IA_SettingsY.IA_SettingsY"))
  (:Started
    (CallFunction|SetSettingsY true))
  (:Canceled
    (CallFunction|SetSettingsY false :!label _label))
  (:Completed
    (goto _label)))

(event Input|EnhancedActionEvents|EnhancedInputActionIA_UseLeft
  (params (ActionValue :type Float%20%28double-precision%29) (ElapsedSeconds :type Float%20%28double-precision%29) (TriggeredSeconds :type Float%20%28double-precision%29) (InputAction :type Input%20Action%20Object%20Reference :default "/Game/Base/Input/IA_UseLeft.IA_UseLeft"))
  (:Triggered
    (CallFunction|ProcessLeftPointer ActionValue))
  (:Canceled
    (CallFunction|ReleaseLeftPointer :!label _label))
  (:Completed
    (goto _label)))

(event Input|EnhancedActionEvents|EnhancedInputActionIA_UseRight
  (params (ActionValue :type Float%20%28double-precision%29) (ElapsedSeconds :type Float%20%28double-precision%29) (TriggeredSeconds :type Float%20%28double-precision%29) (InputAction :type Input%20Action%20Object%20Reference :default "/Game/Base/Input/IA_UseRight.IA_UseRight"))
  (:Triggered
    (CallFunction|ProcessRightPointer ActionValue))
  (:Canceled
    (CallFunction|ReleaseRightPointer :!label _label))
  (:Completed
    (goto _label)))

(event EventBeginPlay
  (Input|EnableInput (Game|Player|GetOwningPlayerController))
  (bind _asmain_game_instance (Utilities|Casting|CastToMainGameInstance (Game|GetGameInstance)))
  (Variables|Default|SetSettingsState _asmain_game_instance)
  (Audio|PushSoundMixModifier "/Game/Base/Audio/SM_Settings.SM_Settings")
  (bind _returnvalue (UserInterface|CreateWidget "/Game/Base/UI/WBP_Settings.WBP_Settings_C" (Game|Player|GetOwningPlayerController) (Variables|Default|GetSettingsState)))
  (UserInterface|SetWidget (Variables|Default|GetSettingsDisplay) _returnvalue)
  (EventDispatchers|BindEventtoCloseRequested _returnvalue (EventDispatchers|CreateEvent :!event CloseSettings)))

(event EventEndPlay
  (params (EndPlayReason :type EEndPlayReason%20Enum :default "Destroyed"))
  (CallFunction|ReleaseLeftPointer)
  (CallFunction|ReleaseRightPointer)
  (Utilities|Time|ClearTimerbyFunctionName self "ToggleSettings")
  (Audio|PopSoundMixModifier "/Game/Base/Audio/SM_Settings.SM_Settings"))

(fn ConstructionScript)

(fn CloseSettings
  (Collision|SetCollisionEnabled (Variables|Default|GetSettingsDisplay) "NoCollision")
  (Rendering|SetVisibility (Variables|Default|GetSettingsDisplay) false false)
  (Variables|Default|SetbSettingsOpen false))

(fn ToggleSettings
  (bind _returnvalue (Game|Player|GetOwningPlayerController))
  (bind _playercameramanager (Variables|/Script/Engine.PlayerController|GetPlayerCameraManager _returnvalue))
  (bind _returnvalue_2 (Camera|GetCameraRotation _playercameramanager))
  (if (Variables|Default|GetbSettingsOpen)
    (CallFunction|CloseSettings)
    (else
      (Transformation|SetWorldLocationAndRotation (Variables|Default|GetSettingsDisplay) (+ (Camera|GetCameraLocation _playercameramanager) (* (Math|Vector|GetForwardVector _returnvalue_2) (Class|KismetSystemLibrary|MakeLiteralInteger 100))) (Math|Rotator|MakeRotator 0.0 0.0 (+ (.Yaw (Math|Rotator|BreakRotator _returnvalue_2)) (Class|KismetSystemLibrary|MakeLiteralInteger 180))) false false)
      (Rendering|SetVisibility (Variables|Default|GetSettingsDisplay) true false)
      (Collision|SetCollisionEnabled (Variables|Default|GetSettingsDisplay) "QueryOnly")
      (Variables|Default|SetbSettingsOpen true))))

(fn UpdateSettingsChord
  (bind _self self)
  (if (and (Variables|Default|GetbSettingsXPressed) (Variables|Default|GetbSettingsYPressed))
    (Utilities|Time|SetTimerbyFunctionName _self "ToggleSettings" 0.6)
    (else
      (Utilities|Time|ClearTimerbyFunctionName _self "ToggleSettings"))))

(fn SetSettingsX
  (params (bPressed :type Boolean))
  (Variables|Default|SetbSettingsXPressed bPressed)
  (CallFunction|UpdateSettingsChord))

(fn SetSettingsY
  (params (bPressed :type Boolean))
  (Variables|Default|SetbSettingsYPressed bPressed)
  (CallFunction|UpdateSettingsChord))

(fn ProcessLeftPointer
  (params (Value :type Float%20%28double-precision%29))
  (bind _asvirtual_reality_pawn (Utilities|Casting|CastToVirtualRealityPawn (Pawn|GetControlledPawn (Game|Player|GetOwningPlayerController))))
  (if (Class|VirtualRealityPawn|IsHandBusy _asvirtual_reality_pawn true)
    (Class|WidgetInteractionComponent|ReleasePointerKey (Variables|/Script/YakutSimulator.VirtualRealityPawn|GetLeftPointer _asvirtual_reality_pawn) "LeftMouseButton"))
  (if (and (>= Value (Math|Float|MakeLiteralFloat 0.65)) (not (Variables|Default|GetbLeftTriggerPressed)))
    (Variables|Default|SetbLeftTriggerPressed true)
    (if (not (Class|VirtualRealityPawn|IsHandBusy _asvirtual_reality_pawn true))
      (if (Class|WidgetInteractionComponent|IsOverHitTestVisibleWidget (Variables|/Script/YakutSimulator.VirtualRealityPawn|GetLeftPointer _asvirtual_reality_pawn))
        (Class|WidgetInteractionComponent|PressPointerKey (Variables|/Script/YakutSimulator.VirtualRealityPawn|GetLeftPointer _asvirtual_reality_pawn) "LeftMouseButton")))
    (elif (and (<= Value (Math|Float|MakeLiteralFloat 0.35)) (Variables|Default|GetbLeftTriggerPressed))
      (Variables|Default|SetbLeftTriggerPressed false)
      (Class|WidgetInteractionComponent|ReleasePointerKey (Variables|/Script/YakutSimulator.VirtualRealityPawn|GetLeftPointer _asvirtual_reality_pawn) "LeftMouseButton"))))

(fn ReleaseLeftPointer
  (CallFunction|ProcessLeftPointer 0.0))

(fn ProcessRightPointer
  (params (Value :type Float%20%28double-precision%29))
  (bind _asvirtual_reality_pawn (Utilities|Casting|CastToVirtualRealityPawn (Pawn|GetControlledPawn (Game|Player|GetOwningPlayerController))))
  (if (Class|VirtualRealityPawn|IsHandBusy _asvirtual_reality_pawn false)
    (Class|WidgetInteractionComponent|ReleasePointerKey (Variables|/Script/YakutSimulator.VirtualRealityPawn|GetRightPointer _asvirtual_reality_pawn) "LeftMouseButton"))
  (if (and (>= Value (Math|Float|MakeLiteralFloat 0.65)) (not (Variables|Default|GetbRightTriggerPressed)))
    (Variables|Default|SetbRightTriggerPressed true)
    (if (not (Class|VirtualRealityPawn|IsHandBusy _asvirtual_reality_pawn false))
      (if (Class|WidgetInteractionComponent|IsOverHitTestVisibleWidget (Variables|/Script/YakutSimulator.VirtualRealityPawn|GetRightPointer _asvirtual_reality_pawn))
        (Class|WidgetInteractionComponent|PressPointerKey (Variables|/Script/YakutSimulator.VirtualRealityPawn|GetRightPointer _asvirtual_reality_pawn) "LeftMouseButton")))
    (elif (and (<= Value (Math|Float|MakeLiteralFloat 0.35)) (Variables|Default|GetbRightTriggerPressed))
      (Variables|Default|SetbRightTriggerPressed false)
      (Class|WidgetInteractionComponent|ReleasePointerKey (Variables|/Script/YakutSimulator.VirtualRealityPawn|GetRightPointer _asvirtual_reality_pawn) "LeftMouseButton"))))

(fn ReleaseRightPointer
  (CallFunction|ProcessRightPointer 0.0))